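; BP_ShroudScout is a Shroud Map actor that circles a center point on a horizontal orbit at constant height.
; Each Tick computes its position with sine and cosine from orbit center, radius, speed and a phase offset in degrees, then sets it without sweeping.
; The angle derives from absolute game time rather than accumulated deltas, so the motion is stateless and independent of frame rate.
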(event `self.ReceiveTick`
  (params (DeltaSeconds :type "Float (single-precision)"))
  (bind _orbitcenter (`self.OrbitCenter`))
  (bind _orbitradius (`self.OrbitRadius`))
  (bind _returnvalue (+ (`self.PhaseDegrees`) (* (`KismetSystemLibrary.GetGameTimeInSeconds`) (`self.OrbitSpeed`))))
  (`self.K2_SetActorLocation` (`KismetMathLibrary.MakeVector` (+ (.x _orbitcenter) (* _orbitradius (`KismetMathLibrary.DegCos` _returnvalue))) (+ (.y _orbitcenter) (* _orbitradius (`KismetMathLibrary.DegSin` _returnvalue))) (.z _orbitcenter))))

(fn `UserConstructionScript`)